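; BP_Char is a player character with free-look camera movement and jumping on Space.
; Forward and Strafe axes offset the actor along the camera's forward and right vectors at a fixed, delta-time-scaled speed without sweep, bypassing collision and movement-component walking.
; Mouse X yaws the X component and Mouse Y pitches the Camera locally, splitting look rotation across two components.
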(event `Key|SpaceBar`
  (params (Key :type "Key Structure" :default "AnyKey"))
  (:`Pressed`
    (`self.Jump`)))

(event `InputAxis|Forward`
  (params (AxisValue :type "Float (single-precision)"))
  (`self.K2_AddActorWorldOffset` (* (`SceneComponent.GetForwardVector` (`self.Camera`)) (* (* AxisValue 500.0) (`GameplayStatics.GetWorldDeltaSeconds`)))))

(event `InputAxis|Strafe`
  (params (AxisValue :type "Float (single-precision)"))
  (`self.K2_AddActorWorldOffset` (* (`SceneComponent.GetRightVector` (`self.Camera`)) (* (* AxisValue 500.0) (`GameplayStatics.GetWorldDeltaSeconds`)))))

(event `InputAxisKey|MouseX`
  (params (AxisValue :type "Float (single-precision)"))
  (`SceneComponent.K2_AddLocalRotation` (`self.X`) (`KismetMathLibrary.MakeRotator` 0.0 0.0 (* (* AxisValue (`GameplayStatics.GetWorldDeltaSeconds`)) 100.0)) false false))

(event `InputAxisKey|MouseY`
  (params (AxisValue :type "Float (single-precision)"))
  (`SceneComponent.K2_AddLocalRotation` (`self.Camera`) (`KismetMathLibrary.MakeRotator` 0.0 (* (* AxisValue (`GameplayStatics.GetWorldDeltaSeconds`)) 100.0)) false false))

(fn `UserConstructionScript`)