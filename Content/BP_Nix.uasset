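; BP_Nix is an audio Blueprint that layers three looping sounds, shaped by how far the player looks up or down.
; On BeginPlay, parallel Delay loops retrigger Kick at a fixed beat, Foutain faster with steeper camera pitch, and Bikes on randomized intervals.
; Absolute camera pitch from BP_Char sets pitch multiplier and start offset for Foutain and Bikes.
; An alternate pitch-driven Kick loop and a random Bikes branch are left unconnected.
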(event `self.ReceiveBeginPlay`
  (bind _foutain (`self.Foutain`))
  (bind _bikes (`self.Bikes`))
  (bind (_returnvalue_roll _returnvalue_pitch) (`KismetMathLibrary.BreakRotator` (`SceneComponent.K2_GetComponentRotation` (`/Game/BP_Char.Camera` (cast `/Game/BP_Char` (`GameplayStatics.GetPlayerPawn` 0) :!pure true)))))
  (bind _returnvalue (`KismetMathLibrary.Abs` (/ _returnvalue_pitch 90.0)))
  (`|ExecutionSequence`
    (:`then_0`
      (`AudioComponent.Play` (`self.Kick`) 0.0 :!label _label)
      (`KismetSystemLibrary.Delay` 0.5)
      (goto _label))
    (:`then_1`
      (`AudioComponent.SetPitchMultiplier` _foutain (+ (* _returnvalue 0.5) 1.5) :!label _label_2)
      (`AudioComponent.Play` _foutain (+ (* _returnvalue 40.0) 5.0))
      (`KismetSystemLibrary.Delay` (* (- 1.0 _returnvalue) 0.2))
      (goto _label_2))
    (:`then_2`
      (`AudioComponent.SetPitchMultiplier` _bikes (+ (* _returnvalue 1.6) 0.4) :!label _label_3)
      (`AudioComponent.Play` _bikes (+ (* _returnvalue 1.0) 7.0))
      (`KismetSystemLibrary.Delay` (select `bool` (`KismetMathLibrary.RandomBoolWithWeight` 0.1) :`false` 0.25 :`true` (select `bool` (`KismetMathLibrary.RandomBool`) :`false` 0.125 :`true` 0.5 :!type "Float (single-precision)")))
      (goto _label_3))))

(fn `UserConstructionScript`)